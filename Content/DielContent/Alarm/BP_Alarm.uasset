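; Alarm light actor that shows rotating red warning beacons while active.
; SetAlarmActive stores the active flag, swaps the alarm mesh between glowing and plain red materials, and toggles visibility of two spotlights, two light beams and a sphere.
; While active, Tick spins the spotlights in yaw and the beams in opposite-signed roll at Speed, scaled by delta time.
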(event EventTick
  (params (DeltaSeconds :type Float%20%28single-precision%29))
  (bind _speed (Variables|Default|GetSpeed))
  (if (Variables|Default|GetIsActive)
    (Transformation|AddLocalRotation (Variables|Default|GetSpotLight1) (* (Math|Rotator|MakeRotator 0.0 0.0 _speed) DeltaSeconds) false false)
    (Transformation|AddLocalRotation (Variables|Default|GetLightBeam1) (* (Math|Rotator|MakeRotator (* _speed -1.0) 0.0 0.0) DeltaSeconds) false false)))

(fn ConstructionScript)

(fn SetAlarmActive
  (params (isActive :type Boolean))
  (bind _alarm (Variables|Default|GetAlarm))
  (bind _spotlight1 (Variables|Default|GetSpotLight1))
  (bind _spotlight2 (Variables|Default|GetSpotLight2))
  (bind _lightbeam1 (Variables|Default|GetLightBeam1))
  (bind _lightbeam2 (Variables|Default|GetLightBeam2))
  (bind _sphere (Variables|Default|GetSphere))
  (bind _output_get (Variables|Default|SetIsActive isActive))
  (if _output_get
    (Rendering|Material|SetMaterial _alarm 0 "/Game/DielContent/Alarm/M_Alarm_RedLight_Glow.M_Alarm_RedLight_Glow")
    (Rendering|SetVisibility _spotlight1 true false)
    (Rendering|SetVisibility _spotlight2 true false)
    (Rendering|SetVisibility _lightbeam1 true false)
    (Rendering|SetVisibility _lightbeam2 true false)
    (Rendering|SetVisibility _sphere true false)
    (else
      (Rendering|Material|SetMaterial _alarm 0 "/Game/DielContent/Alarm/M_Alarm_RedLight.M_Alarm_RedLight")
      (Rendering|SetVisibility _spotlight1 false false)
      (Rendering|SetVisibility _spotlight2 false false)
      (Rendering|SetVisibility _lightbeam1 false false)
      (Rendering|SetVisibility _lightbeam2 false false)
      (Rendering|SetVisibility _sphere false false))))