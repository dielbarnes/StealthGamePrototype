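; Interactable detector that highlights the object ahead of a referenced actor and shows a key/action prompt above it.
; Each Tick a forward sphere trace tracks the current hit, toggling custom depth on its "outline"-tagged component for a post-process outline material.
; Stealable, hackable or pickup tags set outline color and prompt styling.
; The prompt requires a visible static mesh actor, checking the mapped actor for encased stealables.
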(event EventTick
  (params (DeltaSeconds :type Float%20%28single-precision%29))
  (bind _actor (Variables|Default|GetActor))
  (bind _widget (Variables|Default|GetWidget))
  (bind _rootcomponent (Variables|/Script/Engine.Actor|GetRootComponent _actor))
  (bind _returnvalue (Transformation|GetWorldLocation _rootcomponent))
  ;[1 1 1] Outline
  (bind (_outhit _returnvalue_2) (Collision|SphereTraceForObjects _returnvalue (+ _returnvalue (* (Math|Vector|GetForwardVector (Variables|/Script/Engine.Actor|GetRootComponent _actor)) (Variables|Default|Getrange))) (Variables|Default|Getradius) (Utilities|Array|MakeArray "ObjectTypeQuery7") false 0 "None"))
  (if _returnvalue_2
    (if (== (.hitactor (Variables|Default|GetCurrentInteractable)) 0) ; If (sphere trace has a hit) { Check if CurrentInteractable is null }
      (CallFunction|SetOutline (.HitActor (Collision|BreakHitResult _outhit)) true :!label _label) ; Add outline to sphere trace hit
      (Variables|Default|SetCurrentInteractable _outhit) ; Set sphere trace hit as CurrentInteractable
      (CallFunction|SetColorandText)
      ;[1 1 1] Text
      (bind _isvisible (CallFunction|IsVisible (.HitActor (Collision|BreakHitResult _outhit))))
      (if (and _isvisible (Variables|Default|GetShouldShowText))
        (Transformation|SetWorldLocation _widget (+ (Transformation|GetWorldLocation (.HitComponent (Collision|BreakHitResult _outhit))) (Math|Vector|MakeVector 0.0 0.0 (+ (Variables|Default|GetTextZOffset) (.z (.BoxExtent (Collision|GetActorBounds (.HitActor (Collision|BreakHitResult _outhit)) false)))))) false false)
        (bind _asw_interactable (Utilities|Casting|CastToW_Interactable (UserInterface|GetUserWidgetObject _widget)))
        (Rendering|Components|TextRender|SetText (Variables|/Game/DielContent/Interactable/W_Interactable.W_Interactable_C|GetKey _asw_interactable) (Variables|Default|GetKey))
        (Appearance|SetColorandOpacity (Variables|/Game/DielContent/Interactable/W_Interactable.W_Interactable_C|GetKey _asw_interactable) (Utilities|Struct|MakeSlateColor (Math|Conversions|ToLinearColor(Color) (Variables|Default|GetKeyColor))) :!class /Script/UMG.TextBlock)
        (Rendering|Components|TextRender|SetText (Variables|/Game/DielContent/Interactable/W_Interactable.W_Interactable_C|GetAction _asw_interactable) (Variables|Default|GetAction))
        (Appearance|SetColorandOpacity (Variables|/Game/DielContent/Interactable/W_Interactable.W_Interactable_C|GetAction _asw_interactable) (Utilities|Struct|MakeSlateColor (Math|Conversions|ToLinearColor(Color) (Variables|Default|GetActionColor))) :!class /Script/UMG.TextBlock)
        (Rendering|SetVisibility _widget true false))
      (elif (not (== (.hitactor (Variables|Default|GetCurrentInteractable)) (.HitActor (Collision|BreakHitResult _outhit)))) ; If (CurrentInteractable != null) { Check if the sphere trace hit is the CurrentInteractable }
        (CallFunction|SetOutline (.hitactor (Variables|Default|GetCurrentInteractable)) false) ; If (sphere trace hit != CurrentInteractable) { Remove outline of CurrentInteractable }
        (goto _label)))
    (elif (not (== (.hitactor (Variables|Default|GetCurrentInteractable)) 0)) ; If (sphere trace has NO hit) { Check if CurrentInteractable is null }
      (CallFunction|SetOutline (.hitactor (Variables|Default|GetCurrentInteractable)) false) ; If (CurrentInteractable != null) { Remove outline of CurrentInteractable }
      (Variables|Default|SetCurrentInteractable "") ; Set CurrentInteractable to null
      (Rendering|SetVisibility _widget false false))))

(event EventBeginPlay
  ;[1 1 1] Text
  (Rendering|SetVisibility (Variables|Default|GetWidget) false false))

(fn ConstructionScript
  ;[1 1 1] Create Outline Material
  (bind _returnvalue (Rendering|Material|CreateDynamicMaterialInstance "/Game/DielContent/Interactable/M_InteractableOutline.M_InteractableOutline" "" :!class /Script/Engine.KismetMaterialLibrary))
  (bind _output_get (Variables|Default|SetOutlineMaterial _returnvalue))
  (Rendering|AddorUpdateBlendable (Variables|Default|GetPostProcessVolume) _output_get 1.0 :!class /Script/Engine.PostProcessVolume)
  (Rendering|Material|SetVectorParameterValue _output_get "OutlineColor" (Math|Color|MakeColor 0.104904 0.0 0.346875 0.7) :!class /Script/Engine.MaterialInstanceDynamic))

(fn SetOutline
  (params (Interactable :type Actor%20Object%20Reference) (Active :type Boolean))
  (Rendering|SetRenderCustomDepth (Utilities|Array|Get(acopy) (Actor|GetComponentsbyTag Interactable "/Script/Engine.PrimitiveComponent" "outline")) Active))

(fn SetColorandText
  (bind _currentinteractable (Variables|Default|GetCurrentInteractable))
  (bind _outlinematerial (Variables|Default|GetOutlineMaterial))
  (bind _hitcomponent (Collision|BreakHitResult _currentinteractable))
  (if (Components|ComponentHasTag _hitcomponent "stealable")
    (Rendering|Material|SetVectorParameterValue _outlinematerial "OutlineColor" (Math|Conversions|ToLinearColor(Color) (Variables|Default|GetStealableOutlineColor)) :!class /Script/Engine.MaterialInstanceDynamic)
    (Variables|Default|SetKey (Variables|Default|GetStealableKey))
    (Variables|Default|SetKeyColor (Variables|Default|GetStealableKeyColor))
    (Variables|Default|SetAction (Variables|Default|GetStealableAction))
    (Variables|Default|SetActionColor (Variables|Default|GetStealableActionColor))
    (elif (Components|ComponentHasTag _hitcomponent "hackable")
      (Rendering|Material|SetVectorParameterValue _outlinematerial "OutlineColor" (Math|Conversions|ToLinearColor(Color) (Variables|Default|GetHackableOutlineColor)) :!class /Script/Engine.MaterialInstanceDynamic)
      (Variables|Default|SetKey (Variables|Default|GetHackableKey))
      (Variables|Default|SetKeyColor (Variables|Default|GetHackableKeyColor))
      (Variables|Default|SetAction (Variables|Default|GetHackableAction))
      (Variables|Default|SetActionColor (Variables|Default|GetHackableActionColor))
      (elif (Components|ComponentHasTag _hitcomponent "pickup")
        (Rendering|Material|SetVectorParameterValue _outlinematerial "OutlineColor" (Math|Conversions|ToLinearColor(Color) (Variables|Default|GetPickupOutlineColor)) :!class /Script/Engine.MaterialInstanceDynamic)
        (Variables|Default|SetKey (Variables|Default|GetPickupKey))
        (Variables|Default|SetKeyColor (Variables|Default|GetPickupKeyColor))
        (Variables|Default|SetAction (Variables|Default|GetPickupAction))
        (Variables|Default|SetActionColor (Variables|Default|GetPickupActionColor))))))

(fn RemoveText
  (Rendering|SetVisibility (Variables|Default|GetWidget) false false))

(fn IsVisible
  (params (Actor :type Actor%20Object%20Reference))
  (bind _asstatic_mesh_actor (Utilities|Casting|CastToStaticMeshActor Actor))
  (if (.ReturnValue (Utilities|Map|Find (Variables|Default|GetEncasedStealables) _asstatic_mesh_actor))
    (return (Rendering|IsVisible (Variables|/Script/Engine.Actor|GetRootComponent (.Value (Utilities|Map|Find (Variables|Default|GetEncasedStealables) _asstatic_mesh_actor)))))
    (else
      (return (Rendering|IsVisible (Variables|/Script/Engine.Actor|GetRootComponent _asstatic_mesh_actor))))))