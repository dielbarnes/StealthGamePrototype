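; BP_Laser is a laser obstacle that reports when a designated actor touches its beam and can optionally move or blink.
; On BeginPlay a forward line trace sets the beam end, then it spawns the particle beam, stretches the collision box and places the end emitter.
; Timelines slide the whole assembly along an axis or toggle beam visibility with collision.
; Overlap stores the actor's location and fires a dispatcher; DisableLaser hides the beam and turns the emitter lights red.
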(event OnComponentBeginOverlap(CollisionBox)
  (params (OverlappedComponent :type Primitive%20Component%20Object%20Reference) (OtherActor :type Actor%20Object%20Reference) (OtherComp :type Primitive%20Component%20Object%20Reference) (OtherBodyIndex :type Integer) (bFromSweep :type Boolean) (SweepResult :type Hit%20Result%20Structure%20%28by%20ref%29))
  (bind _actor (Variables|Default|GetActor))
  ;[1 1 1] Collision Event
  (if (== OtherActor _actor)
    (Variables|Default|SetLastKnownActorLocation (Transformation|GetWorldLocation (Variables|/Script/Engine.Actor|GetRootComponent _actor)))
    (Default|CallCollisionEventDispatcher self)))

(event Custom|PlayMovement
  (bind _laserparticle (Variables|Default|GetLaserParticle))
  (bind _movement_timeline (Variables|Default|GetMovement%20Timeline))
  ;[1 1 1] Movement
  (Components|Timeline|SetPlayRate _movement_timeline (* (Variables|Default|GetSpeed) (Components|Animation|GetPlayRate _movement_timeline)))
  (bind _movementdistance (Timeline|Movement%20Timeline Play)
    (:Update
      (Transformation|SetWorldLocation (Variables|Default|GetLaserEmitterStart) (+ (* (Variables|Default|GetMovementAxis) (* _movementdistance (Variables|Default|GetMovementDistance))) (Variables|Default|GetLaserEmitterStartInitialLocation)) false false)
      (Transformation|SetWorldLocation _laserparticle (+ (* (Variables|Default|GetMovementAxis) (* _movementdistance (Variables|Default|GetMovementDistance))) (Variables|Default|GetLaserParticleInitialLocation)) false false)
      (Class|ParticleSystemComponent|SetBeamEndPoint _laserparticle 0 (+ (* (Variables|Default|GetMovementAxis) (* _movementdistance (Variables|Default|GetMovementDistance))) (Variables|Default|GetLaserEndPoint)))
      (Transformation|SetWorldLocation (Variables|Default|GetCollisionBox) (+ (* (Variables|Default|GetMovementAxis) (* _movementdistance (Variables|Default|GetMovementDistance))) (Variables|Default|GetCollisionBoxInitialLocation)) false false)
      (Transformation|SetWorldLocation (Variables|Default|GetLaserEmitterEnd) (+ (* (Variables|Default|GetMovementAxis) (* _movementdistance (Variables|Default|GetMovementDistance))) (Variables|Default|GetLaserEmitterEndInitialLocation)) false false))))

(event Custom|StopMovement
  (bind _laserparticle (Variables|Default|GetLaserParticle))
  ;[1 1 1] Movement
  (bind _movementdistance (Timeline|Movement%20Timeline Stop)
    (:Update
      (Transformation|SetWorldLocation (Variables|Default|GetLaserEmitterStart) (+ (* (Variables|Default|GetMovementAxis) (* _movementdistance (Variables|Default|GetMovementDistance))) (Variables|Default|GetLaserEmitterStartInitialLocation)) false false)
      (Transformation|SetWorldLocation _laserparticle (+ (* (Variables|Default|GetMovementAxis) (* _movementdistance (Variables|Default|GetMovementDistance))) (Variables|Default|GetLaserParticleInitialLocation)) false false)
      (Class|ParticleSystemComponent|SetBeamEndPoint _laserparticle 0 (+ (* (Variables|Default|GetMovementAxis) (* _movementdistance (Variables|Default|GetMovementDistance))) (Variables|Default|GetLaserEndPoint)))
      (Transformation|SetWorldLocation (Variables|Default|GetCollisionBox) (+ (* (Variables|Default|GetMovementAxis) (* _movementdistance (Variables|Default|GetMovementDistance))) (Variables|Default|GetCollisionBoxInitialLocation)) false false)
      (Transformation|SetWorldLocation (Variables|Default|GetLaserEmitterEnd) (+ (* (Variables|Default|GetMovementAxis) (* _movementdistance (Variables|Default|GetMovementDistance))) (Variables|Default|GetLaserEmitterEndInitialLocation)) false false))))

(event Custom|PlayBlinking
  (bind _collisionbox (Variables|Default|GetCollisionBox))
  (bind _blinktimeline (Variables|Default|GetBlinkTimeline))
  ;[1 1 1] Blinking
  (Components|Timeline|SetPlayRate _blinktimeline (* (Variables|Default|GetSpeed) (Components|Animation|GetPlayRate _blinktimeline)))
  (bind _visibility (Timeline|BlinkTimeline Play)
    (:Update
      (Rendering|SetVisibility (Variables|Default|GetLaserParticle) (Math|Conversions|ToBoolean(Integer) (Math|Float|Truncate _visibility)) false)
      (if (Math|Conversions|ToBoolean(Integer) (Math|Float|Truncate _visibility))
        (Collision|SetCollisionEnabled _collisionbox "QueryAndPhysics")
        (else
          (Collision|SetCollisionEnabled _collisionbox "NoCollision"))))))

(event Custom|StopBlinking
  (bind _collisionbox (Variables|Default|GetCollisionBox))
  ;[1 1 1] Blinking
  (bind _visibility (Timeline|BlinkTimeline Stop)
    (:Update
      (Rendering|SetVisibility (Variables|Default|GetLaserParticle) (Math|Conversions|ToBoolean(Integer) (Math|Float|Truncate _visibility)) false)
      (if (Math|Conversions|ToBoolean(Integer) (Math|Float|Truncate _visibility))
        (Collision|SetCollisionEnabled _collisionbox "QueryAndPhysics")
        (else
          (Collision|SetCollisionEnabled _collisionbox "NoCollision"))))))

(event EventBeginPlay
  (bind _laserstartpoint (Variables|Default|GetLaserStartPoint))
  (bind _laseremitterend (Variables|Default|GetLaserEmitterEnd))
  (bind _collisionbox (Variables|Default|GetCollisionBox))
  (bind _returnvalue (Transformation|GetWorldLocation _laserstartpoint))
  (bind _returnvalue_2 (Transformation|GetWorldLocation _laseremitterend))
  ;[1 1 1] Create Beam + Collision Box
  (Variables|Default|SetLaserEmitterStartInitialLocation (Transformation|GetWorldLocation (Variables|Default|GetLaserEmitterStart)))
  (Variables|Default|SetLaserParticleInitialLocation (Transformation|GetWorldLocation (Variables|Default|GetLaserStartPoint)))
  (bind _output_get (Variables|Default|SetLaserEndPoint (+ _returnvalue (* (Math|Vector|GetForwardVector _laserstartpoint) (Variables|Default|GetDefaultLength)))))
  (bind (_outhit _returnvalue_3) (Collision|LineTraceByChannel _returnvalue _output_get "TraceTypeQuery1" false 0 "None"))
  (if _returnvalue_3
    (bind _output_get_2 (Variables|Default|SetLaserEndPoint (.Location (Collision|BreakHitResult _outhit)))))
  (CallFunction|CreateBeam _returnvalue _output_get_2)
  (CallFunction|ScaleCollisionBox _output_get_2)
  (Variables|Default|SetCollisionBoxInitialLocation (Transformation|GetWorldLocation _collisionbox))
  (Collision|SetCollisionEnabled _collisionbox "QueryAndPhysics")
  (Transformation|AddLocalOffset _laseremitterend "0,-60.000000,0.000000" false false)
  (Transformation|SetWorldLocation _laseremitterend (+ _returnvalue_2 (- _output_get_2 _returnvalue)) false false)
  (Variables|Default|SetLaserEmitterEndInitialLocation _returnvalue_2))

(fn ConstructionScript)

(fn CreateBeam
  (params (StartPoint :type Vector) (EndPoint :type Vector))
  (bind _returnvalue (Effects|SpawnEmitteratLocation "/Game/DielContent/Laser/P_Laser.P_Laser" StartPoint))
  (bind _output_get (Variables|Default|SetLaserParticle _returnvalue))
  (Class|ParticleSystemComponent|SetBeamEndPoint _output_get 0 EndPoint))

(fn ScaleCollisionBox
  (params (EndPoint :type Vector))
  (bind _laserstartpoint (Variables|Default|GetLaserStartPoint))
  (bind _collisionbox (Variables|Default|GetCollisionBox))
  (bind _returnvalue (Transformation|GetWorldLocation _laserstartpoint))
  (bind _returnvalue_2 (- EndPoint _returnvalue))
  (bind _returnvalue_3 (/ _returnvalue_2 2.0))
  (Transformation|SetRelativeScale3D _collisionbox (Math|Vector|MakeVector (Math|Vector|VectorLength _returnvalue_3) 1.0 1.0))
  (Transformation|SetWorldLocation _collisionbox (+ (Transformation|GetWorldLocation _collisionbox) _returnvalue_3) false false))

(fn DisableLaser
  (Rendering|SetVisibility (Variables|Default|GetLaserParticle) false false)
  (Collision|SetCollisionEnabled (Variables|Default|GetCollisionBox) "NoCollision")
  (Rendering|Material|SetMaterial (Variables|Default|GetLaserEmitterStart) 1 "/Game/DielContent/Laser/M_LaserEmitter_RedLight.M_LaserEmitter_RedLight")
  (Rendering|Material|SetMaterial (Variables|Default|GetLaserEmitterEnd) 1 "/Game/DielContent/Laser/M_LaserEmitter_RedLight.M_LaserEmitter_RedLight")
  (if (Audio|Components|Audio|IsPlaying (Variables|Default|GetMovement%20Timeline))
    (CallFunction|StopMovement)
    (elif (Audio|Components|Audio|IsPlaying (Variables|Default|GetBlinkTimeline))
      (CallFunction|StopBlinking))))