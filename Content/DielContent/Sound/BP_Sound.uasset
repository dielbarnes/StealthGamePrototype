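; BP_Sound is a sound manager Blueprint that holds the game's music and event sounds for a stealth game with treasures and levels.
; It starts the stealth theme on BeginPlay, and PlayAlarmTheme swaps it for the alarm theme unless that is already playing.
; Simple functions play the game over, level complete, major treasure and minor treasure sounds from the start when called.
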(event EventBeginPlay
  (Audio|Components|Audio|Play (Variables|Default|GetStealthTheme) 0.0))

(fn ConstructionScript)

(fn PlayAlarmTheme
  (bind _alarmtheme (Variables|Default|GetAlarmTheme))
  (if (not (Audio|Components|Audio|IsPlaying _alarmtheme))
    (Audio|Components|Audio|Stop (Variables|Default|GetStealthTheme))
    (Audio|Components|Audio|Play _alarmtheme 0.0)))

(fn PlayGameOverSound
  (Audio|Components|Audio|Play (Variables|Default|GetGameOverSound) 0.0))

(fn PlayLevelCompleteSound
  (Audio|Components|Audio|Play (Variables|Default|GetLevelCompleteSound) 0.0))

(fn PlayMajorTreasureSound
  (Audio|Components|Audio|Play (Variables|Default|GetMajorTreasureSound) 0.0))

(fn PlayMinorTreasureSound
  (Audio|Components|Audio|Play (Variables|Default|GetMinorTreasureSound) 0.0))