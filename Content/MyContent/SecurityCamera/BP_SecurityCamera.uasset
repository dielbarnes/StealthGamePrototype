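; Security camera actor that sweeps its view and reports when a designated actor enters its detection cone.
; On BeginPlay, a timeline with its play rate scaled by Speed drives the camera's world rotation around its up vector.
; When the collision cone begins overlapping the tracked Actor, it stores that actor's last known location and fires an event dispatcher, passing itself to listeners.
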(event OnComponentBeginOverlap(CollisionCone)
  (params (OverlappedComponent :type Primitive%20Component%20Object%20Reference) (OtherActor :type Actor%20Object%20Reference) (OtherComp :type Primitive%20Component%20Object%20Reference) (OtherBodyIndex :type Integer) (bFromSweep :type Boolean) (SweepResult :type Hit%20Result%20Structure%20%28by%20ref%29))
  (bind _actor (Variables|Default|GetActor))
  ;[1 1 1] Collision Event
  (if (== OtherActor _actor)
    (Variables|Default|SetLastKnownActorLocation (Transformation|GetWorldLocation (Variables|/Script/Engine.Actor|GetRootComponent _actor)))
    (Default|CallCollisionEventDispatcher self)))

(event EventBeginPlay
  (bind _camera (Variables|Default|GetCamera))
  (bind _rotationtimeline (Variables|Default|GetRotationTimeline))
  ;[1 1 1] Rotation
  (Components|Timeline|SetPlayRate _rotationtimeline (* (Variables|Default|GetSpeed) (Components|Animation|GetPlayRate _rotationtimeline)))
  (bind _angle (Timeline|RotationTimeline Play)
    (:Update
      (Transformation|SetWorldRotation _camera (Math|Vector|RotatorfromAxisandAngle (Math|Vector|GetUpVector _camera) (* _angle 225.0)) false false))))

(fn ConstructionScript)